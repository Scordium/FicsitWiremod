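; BP_ManagedSign is a buildable sign that renders configurable data through a world-space widget.
; GenerateSignWidget renders the ManagedSignRender widget, sizes it from data size and DPI, then configures emission, matte, redraw rate and transparency.
; Mesh and plane optionally scale with the sign.
; Client processing copies the widget's SlateUI render texture into the plane's dynamic material, apparently so the sign emits Lumen light.
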(event EventClientProcess
  (params (DeltaTime :type Float%20%28double-precision%29))
  (|CallParentFunction DeltaTime)
  (bind _returnvalue (Rendering|Material|GetTextureParameterValue (UserInterface|GetMaterialInstance (Variables|Default|GetWidget)) "SlateUI" :!class /Script/Engine.MaterialInstanceDynamic))
  (bind _output_get (Variables|Default|SetSignRenderTexture _returnvalue))
  (Rendering|Material|SetTextureParameterValue (Variables|Default|GetMaterial) "SlateTexture" _output_get))

(fn ConstructionScript
  (CallFunction|SetSizes))

(fn SetSizes
  (bind _data (Variables|Default|GetData))
  (bind _data_2 (Variables|Default|GetData))
  (bind _widget (Variables|Default|GetWidget))
  (bind (_size _dotsperinch) (Utilities|Struct|BreakManagedSignData _data_2))
  (bind _size_2 (Utilities|Struct|BreakManagedSignData _data))
  (bind _returnvalue (Math|Conversions|ToFloat(Integer) _dotsperinch))
  (bind _returnvalue_2 (/ _size_2 "(X=200.000000,Y=200.000000)"))
  (bind _returnvalue_3 (/ _returnvalue 2e+02))
  (bind _returnvalue_4 (/ 1e+02 _returnvalue))
  (Class|WidgetComponent|SetDrawSize _widget (* _size (Math|Vector2D|MakeVector2D _returnvalue_3 _returnvalue_3)))
  (Transformation|SetRelativeScale3D _widget (Math|Vector|MakeVector 1.0 _returnvalue_4 _returnvalue_4))
  (if (Variables|Default|GetShouldSetMeshSize)
    (Transformation|SetRelativeScale3D (Variables|Character|GetMesh) (Math|Vector|MakeVector (.x _returnvalue_2) (.y _returnvalue_2) 0.05))
    (Transformation|SetRelativeScale3D (Variables|Default|GetPlane) (Math|Vector|MakeVector (.x _returnvalue_2) (.y _returnvalue_2) 1.0))))

(fn GenerateLumenLightMaterial
  (bind _returnvalue (Rendering|Material|CreateDynamicMaterialInstance (Variables|Default|GetPlane) 0 "/FicsitWiremod/Buildings/Displays/ManagedSigns/Buildable/ManagedSignSlateRender.ManagedSignSlateRender" "None" :!class /Script/Engine.PrimitiveComponent))
  (Rendering|Material|SetMaterial (Variables|Default|GetPlane) 0 _returnvalue)
  (Variables|Default|SetMaterial _returnvalue))

(fn GenerateSignWidget
  (params (NewData :type Managed%20Sign%20Data%20Structure%20%28by%20ref%29))
  (Utilities|FlowControl|Sequence
    (:then_0
      (|GenerateWidgetComponents))
    (:then_1
      (CallFunction|SetSizes))
    (:then_2
      (CallFunction|GenerateLumenLightMaterial))
    (:then_3
      (|ConfigureRenderer))))