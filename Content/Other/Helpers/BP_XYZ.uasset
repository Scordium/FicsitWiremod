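; BP_XYZ is a helper actor that shows a marker mesh on a target actor and hides it when no valid target is given.
; SetPosition places the mesh at the target's actor location, or at its bounds center while ToObjectCenter is set.
; ToObjectCenter is true only while the FicsitWiremod SpecialAction input is held.
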(event Input|ActionEvents|InputActionFicsitWiremod.SpecialAction
  (params (Key :type Key%20Structure :default "None"))
  (:Pressed
    (Variables|Default|SetToObjectCenter true))
  (:Released
    (Variables|Default|SetToObjectCenter false)))

(fn ConstructionScript)

(fn SetPosition
  (params (Target :type Actor%20Object%20Reference))
  (if (Utilities|IsValid Target)
    (Transformation|SetWorldLocation (Variables|Default|GetStaticMesh) (select (Variables|Default|GetToObjectCenter) (.Origin (Collision|GetActorBounds Target false true)) (Transformation|GetActorLocation Target)) false false)
    (Development|SetHiddeninGame (Variables|Default|GetStaticMesh) false false)
    (else
      (Development|SetHiddeninGame (Variables|Default|GetStaticMesh) true false))))